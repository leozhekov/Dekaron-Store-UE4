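; Player character for a store scene that can inspect a picked-up item.
; While Inspect is held on a valid picked actor, Turn and LookUp input yaw and pitch that actor instead of the camera.
; TurnObject and RollObject apply the inverted, scaled-down input by combining rotators.
; Widget creation and logic for pick-up, inspect, drop and leave prompts remains in the graph but is disconnected, so it never runs.
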(event EventTick
  (params (DeltaSeconds :type Float%20%28single-precision%29)))

(event EventBeginPlay)

(event Input|ActionEvents|InputActionInspect
  (params (Key :type Key%20Structure))
  ;[1 1 1] Inspecting
  (:Pressed
    (bind _returnvalue (Class|DkrStoreCharacter|PickedActor))
    (Utilities|IsValid _returnvalue
      (:Is%20Valid
        (Variables|Default|SetCurrentlyPickedActor _returnvalue)
        (Variables|Default|SetIsInspecting true))
      (:Is%20Not%20Valid
        (Variables|Default|SetIsInspecting false :!label _label))))
  (:Released
    (Variables|Default|SetCurrentlyPickedActor 0)
    (goto _label)))

(event Input|AxisEvents|InputAxisTurn
  (params (AxisValue :type Float%20%28single-precision%29))
  (if (Variables|Default|GetIsInspecting)
    (CallFunction|TurnObject AxisValue)
    (else
      (Pawn|Input|AddControllerYawInput AxisValue))))

(event Input|AxisEvents|InputAxisLookUp
  (params (AxisValue :type Float%20%28single-precision%29))
  (if (Variables|Default|GetIsInspecting)
    (CallFunction|RollObject AxisValue)
    (else
      (Pawn|Input|AddControllerPitchInput AxisValue))))

(fn ConstructionScript)

(fn TurnObject
  (params (Yaw :type Float%20%28single-precision%29))
  (Transformation|SetActorRotation (Variables|Default|GetCurrentlyPickedActor) (Math|Rotator|CombineRotators (Math|Rotator|MakeRotator 0.0 0.0 (/ (* -1 Yaw) 1e+01)) (Transformation|GetActorRotation (Variables|Default|GetCurrentlyPickedActor)))))

(fn RollObject
  (params (Pitch :type Float%20%28single-precision%29))
  (Transformation|SetActorRotation (Variables|Default|GetCurrentlyPickedActor) (Math|Rotator|CombineRotators (Math|Rotator|MakeRotator 0.0 (/ (* -1 Pitch) 1e+01) 0.0) (Transformation|GetActorRotation (Variables|Default|GetCurrentlyPickedActor)))))

(fn CreateWidgets
  (bind _returnvalue (UserInterface|CreateWidget "/Game/Blueprints/HUD/PickUp.PickUp_C" (Game|GetPlayerController 0)))
  (Variables|Default|SetPickUpWidget _returnvalue)
  (bind _returnvalue_2 (UserInterface|CreateWidget "/Game/Blueprints/HUD/Inspect.Inspect_C" (Game|GetPlayerController 0)))
  (Variables|Default|SetInspectWidget _returnvalue_2)
  (bind _returnvalue_3 (UserInterface|CreateWidget "/Game/Blueprints/HUD/Drop.Drop_C" (Game|GetPlayerController 0)))
  (Variables|Default|SetDropWidget _returnvalue_3)
  (bind _returnvalue_4 (UserInterface|CreateWidget "/Game/Blueprints/HUD/Leave.Leave_C" (Game|GetPlayerController 0)))
  (Variables|Default|SetLeaveWidget _returnvalue_4))

(fn AddWidgetstoViewport
  (UserInterface|Viewport|AddtoViewport (Variables|Default|GetPickUpWidget) 0)
  (UserInterface|Viewport|AddtoViewport (Variables|Default|GetDropWidget) 0)
  (UserInterface|Viewport|AddtoViewport (Variables|Default|GetLeaveWidget) 0)
  (UserInterface|Viewport|AddtoViewport (Variables|Default|GetInspectWidget) 0))